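; Physics test tube that holds a LiquidUnit, with simulated slosh, pouring and a plug shown when capped.
; While the container's rigid body is awake, it copies the liquid mesh to a procedural mesh and slices it by a plane from fill level and damped inertia.
; When uncapped, outflow follows tilt and liquid height; a downward trace pours into another tube or spills, and a stretched mesh draws the stream.
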(event Custom|Update%20Liquid
  (bind _content (Variables|Default|GetContent))
  (bind _content_2 (Variables|Default|GetContent))
  (bind _capped (Variables|Default|GetCapped))
  (bind _plug (Variables|Default|GetPlug))
  (bind _procedural_liquid (Variables|Default|GetProcedural%20Liquid))
  (bind _pouringliquid (Variables|Default|GetPouringLiquid))
  (bind _exit (Variables|Default|GetExit))
  (bind _materialinstance (Variables|Default|GetMaterialInstance))
  (bind (_origin _boxextent) (Collision|GetComponentBounds _exit))
  (bind _volume (Variables|/Game/Blueprints/LiquidUnit.LiquidUnit_C|GetVolume _content))
  (CallFunction|UpdateLiquidInertia)
  (Utilities|FlowControl|Sequence
    (:then_0
      ;[1 1 1] Slice liquid and update plug
      (Default|UpdateMaterialInstance (Variables|Default|GetContent) _materialinstance)
      (Rendering|Material|SetMaterial (Variables|Default|GetLiquid) 0 _materialinstance)
      (Class|KismetProceduralMeshLibrary|CopyProceduralMeshfromStaticMeshComponent (Variables|Default|GetLiquid) 0 _procedural_liquid false)
      (bind (_planeposition _planenormal) (CallFunction|GetLiquidPlane))
      (bind _output_get (Variables|Default|SetPlaneNormal _planenormal))
      (bind _output_get_2 (Variables|Default|SetPlanePosition _planeposition))
      (Class|KismetProceduralMeshLibrary|SliceProceduralMesh _procedural_liquid _output_get_2 _output_get false "UseLastSectionForCap" (Rendering|Material|GetMaterial _procedural_liquid 0))
      (Rendering|SetVisibility _plug _capped false)
      (Collision|SetCollisionEnabled _plug (select _capped "QueryAndPhysics" "NoCollision")))
    (:then_1
      ;[1 1 1] Handle liquid pouring logic
      (Variables|Default|SetLiquidExitPoint (.OutPointOnBody (Collision|GetClosestPointonCollision _exit (- _origin "0, 0,5.000000") "None")))
      (bind _output_get_3 (Variables|Default|SetLiquid%20Outpour (Math|Float|Clamp(Float) (* (* (Math|Conversions|ToFloat(Boolean) (not (Variables|Default|GetCapped))) (|((clamp((max(x,(0-y))),0,1))*pourspeed) (/ (.Z (Math|Vector|BreakVector (- (Variables|Default|GetPlanePosition) (Variables|Default|GetLiquidExitPoint)))) (* (Math|Vector|VectorLength _boxextent) 2.0)) (Math|Float|Clamp(Float) (.Z (Math|Vector|BreakVector (Math|Vector|GetUpVector (Variables|Default|GetExit)))) -1.0 0.0) 1e+03)) (Utilities|Time|GetWorldDeltaSeconds)) (- _volume (Variables|Default|GetCapacity)) _volume)))
      (Rendering|SetVisibility (Variables|Default|GetPouringLiquid) (> _output_get_3 0.0) false)
      (if (> _output_get_3 0.0)
        (bind _outhit (Collision|LineTraceByChannel (Variables|Default|GetLiquidExitPoint) (+ (Variables|Default|GetLiquidExitPoint) "0, 0,-1000.000000") "TraceTypeQuery1" true 0 "None" true "(R=1.000000,G=0.000000,B=0.000000,A=1.000000)" "(R=0.000000,G=0.000000,B=0.000000,A=1.000000)" 0.1))
        (Variables|Default|SetLiquidImpactPoint (.ImpactPoint (Collision|BreakHitResult _outhit)))
        (bind _astest_tube (Utilities|Casting|CastToTestTube (.HitActor (Collision|BreakHitResult _outhit)))
          (:then
            (if (> (Math|Vector|DotProduct (- (.Origin (Collision|GetComponentBounds (Variables|TestTube_C|GetContainer _astest_tube))) (Variables|Default|GetLiquidImpactPoint)) (.ImpactNormal (Collision|BreakHitResult _outhit))) 0.0)
              (Default|PourIntoContainer _content_2 (Variables|TestTube_C|GetContent _astest_tube) (Variables|Default|GetLiquid%20Outpour))
              (CallFunction|UpdateLiquid _astest_tube)
              (else
                (Default|PourOut _content_2 (Variables|Default|GetLiquid%20Outpour) :!label _label))))
          (:CastFailed
            (goto _label)))))
    (:then_2
      ;[1 1 1] Update pouring liquid mesh
      (Rendering|SetVisibility (Variables|Default|GetPouringLiquid) (> (Variables|Default|GetLiquid%20Outpour) 0.0) false)
      (if (> (Variables|Default|GetLiquid%20Outpour) 0.0)
        (Rendering|Material|SetMaterial _pouringliquid 0 (Rendering|Material|GetMaterial (Variables|Default|GetLiquid) 0))
        (Transformation|SetWorldTransform _pouringliquid (Math|Transform|MakeTransform (Math|Vector|Lerp(Vector) (Variables|Default|GetLiquidExitPoint) (Variables|Default|GetLiquidImpactPoint) 0.5) "0, 0, 0" (/ (Math|Vector|MakeVector (* (Math|Float|Sqrt (Variables|Default|GetLiquid%20Outpour)) 0.5) (* (Math|Float|Sqrt (Variables|Default|GetLiquid%20Outpour)) 0.5) (Math|Vector|VectorLength (- (Variables|Default|GetLiquidExitPoint) (Variables|Default|GetLiquidImpactPoint)))) 1e+02)) false false)))))

(event EventTick
  (params (DeltaSeconds :type Float%20%28single-precision%29))
  (if (Class|PrimitiveComponent|IsAnyRigidBodyAwake (Variables|Default|GetContainer))
    (CallFunction|UpdateLiquid)))

(fn ConstructionScript
  (Utilities|IsValid (Variables|Default|GetContent)
    (:Is%20Valid
      _)
    (:Is%20Not%20Valid
      (bind _returnvalue (Game|ConstructObjectfromClass "/Game/Blueprints/LiquidUnit.LiquidUnit_C" self))
      (Variables|Default|SetContent _returnvalue)))
  (bind _returnvalue_2 (Rendering|Material|CreateDynamicMaterialInstance (Variables|Default|GetMaterialInstance) "/Game/Materials/MI_Liquid.MI_Liquid" :!class /Script/Engine.KismetMaterialLibrary))
  (bind _output_get (Variables|Default|SetMaterialInstance _returnvalue_2))
  (Variables|Default|SetLiquidInertia (Transformation|GetWorldLocation (Variables|Default|GetContainer)))
  (Utilities|FlowControl|Sequence
    (:then_0
      (bind _returnvalue_3 (AddComponent|AddProceduralMeshComponent false))
      (bind _output_get_2 (Variables|Default|SetProcedural%20Pour _returnvalue_3))
      (Rendering|Material|SetMaterial _output_get_2 0 _output_get))
    (:then_1
      (bind _returnvalue_4 (AddComponent|AddProceduralMeshComponent false))
      (bind _output_get_3 (Variables|Default|SetProcedural%20Liquid _returnvalue_4))
      (Rendering|Material|SetMaterial _output_get_3 0 _output_get))
    (:then_2
      (CallFunction|UpdateLiquid))))

(fn UpdateLiquidInertia
  (bind _returnvalue (Utilities|Time|GetWorldDeltaSeconds))
  (bind _output_get (Variables|Default|SetLiquidVelocity (/ (+ (* (- (Transformation|GetWorldLocation (Variables|Default|GetContainer)) (Variables|Default|GetLiquidInertia)) (* _returnvalue 1.0)) (Variables|Default|GetLiquidVelocity)) (+ (* _returnvalue 1e+01) 1.0))))
  (Variables|Default|SetLiquidInertia (+ (* _output_get (* _returnvalue 5e+02)) (Variables|Default|GetLiquidInertia)))
  (return))

(fn AddLiquid
  (bind _content (Variables|Default|GetContent))
  (Default|AddConcentrates _content (Variables|Default|GetComponentsToAdd) 1.0)
  (Variables|/Game/Blueprints/LiquidUnit.LiquidUnit_C|SetVolume _content (+ (Variables|/Game/Blueprints/LiquidUnit.LiquidUnit_C|GetVolume _content) 1e+01))
  (CallFunction|UpdateLiquid))

(fn GetLiquidPlane
  (bind _content (Variables|Default|GetContent))
  (bind _liquid_bb_extrusion (Variables|Default|GetLiquid%20BB%20Extrusion))
  (bind _container (Variables|Default|GetContainer))
  (bind _liquid (Variables|Default|GetLiquid))
  (bind _capacity (Variables|Default|GetCapacity))
  (bind _liquidinertia (Variables|Default|GetLiquidInertia))
  (bind (_origin _boxextent) (Collision|GetComponentBounds _liquid))
  (bind _returnvalue (Transformation|GetWorldLocation _container))
  (bind _returnvalue_2 (* _liquid_bb_extrusion -1.0))
  (bind _volume (Variables|/Game/Blueprints/LiquidUnit.LiquidUnit_C|GetVolume _content))
  (bind _returnvalue_3 (- _liquidinertia _returnvalue))
  (bind _returnvalue_4 (/ _volume _capacity))
  (bind _returnvalue_5 (- _returnvalue_3 "0,0.000000,10.000000"))
  (bind (_x _y _z) (Math|Vector|BreakVector _returnvalue_5))
  (return (+ _origin (* _boxextent (* (Math|Vector|MakeVector (Math|Float|Clamp(Float) _x _returnvalue_2 _liquid_bb_extrusion) (Math|Float|Clamp(Float) _y -1.0 _liquid_bb_extrusion) (Math|Float|Clamp(Float) _z _returnvalue_2)) (+ (* (Math|Float|Clamp(Float) _returnvalue_4 _returnvalue_2 _liquid_bb_extrusion) -2.0) 1.0)))) (Math|Vector|Normalize (Math|Vector|Lerp(Vector) "0, 0,-1.000000" _returnvalue_5 _returnvalue_4))))

(fn PrintContent
  (Default|PrintContent (Variables|Default|GetContent)))