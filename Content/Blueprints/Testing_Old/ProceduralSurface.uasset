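; Procedural floor surface actor that tiles a plane's bounds with instanced pavement meshes, built either in the construction script or on BeginPlay.
; Creates one instanced mesh component per floor mesh, counter-scaled against the plane, and stretches grid spacing to fit the bounds exactly.
; World-space simplex noise sets a Destruction value that, with random jitter, picks each tile's mesh variant and scales its yaw jitter.
; Tiles also get random quarter turns and scale variation.
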(event `Build`
  (bind _spacing (`self.Spacing`))
  (bind _floor_isms (`self.Floor ISMs`))
  (bind _jitter (`self.Jitter`))
  (bind _plane (`self.Plane`))
  (bind _scale_jitter (`self.Scale Jitter`))
  (bind _returnvalue (`KismetArrayLibrary.Array_Length` _floor_isms))
  (bind (_min _max) (`StaticMeshComponent.GetLocalBounds` _plane))
  (bind _returnvalue_2 (`SceneComponent.K2_GetComponentScale` _plane))
  (bind _returnvalue_3 (* (`self.Destruction`) (`self.Yaw Jitter`)))
  (bind _returnvalue_4 (- (.y (/ (+ (* (* _min _returnvalue_2) -1.0) (* _max _returnvalue_2)) (`self.Spacing`))) 1.0))
  (bind _returnvalue_5 (- (.x (/ (+ (* (* _min _returnvalue_2) -1.0) (* _max _returnvalue_2)) (`self.Spacing`))) 1.0))
  (bind _returnvalue_6 (`KismetMathLibrary.FTrunc` _returnvalue_5))
  (bind _returnvalue_7 (`KismetMathLibrary.FTrunc` _returnvalue_4))
  (for _array_element (`self.Floor Meshes`) :!label _label
    (bind _returnvalue_8 (`AddComponent|NODE_AddInstancedStaticMeshComponent-3` :`RelativeTransform` (`KismetMathLibrary.InvertTransform` (`KismetMathLibrary.MakeTransform` (0.0 0.0 0.0) (struct) _returnvalue_2))))
    (`StaticMeshComponent.SetStaticMesh` _returnvalue_8 _array_element)
    (`PrimitiveComponent.SetMaterial` _returnvalue_8 0 "/Game/Materials/Dungeon_Pavement.Dungeon_Pavement")
    (`KismetArrayLibrary.Array_Add` (`self.Floor ISMs`) _returnvalue_8))
  (for _index (range (+ _returnvalue_6 1))
    (for _index_2 (range (+ _returnvalue_7 1))
      (bind _returnvalue_9 (+ (* (+ (0.5 0.5 0.0) (`KismetMathLibrary.MakeVector` (`KismetMathLibrary.Conv_IntToDouble` _index) (`KismetMathLibrary.Conv_IntToDouble` _index_2))) (`KismetMathLibrary.MakeVector` (+ (* (/ (mod _returnvalue_5 1.0) (`KismetMathLibrary.Conv_IntToDouble` (+ _returnvalue_6 1))) _spacing) _spacing) (+ _spacing (* _spacing (/ (mod _returnvalue_4 1.0) (`KismetMathLibrary.Conv_IntToDouble` (+ _returnvalue_7 1))))))) (* _min _returnvalue_2)))
      (bind _returnvalue_10 (`SimplexNoise.SimplexNoise` (/ (+ (`SceneComponent.K2_GetComponentLocation` (`self.Plane`)) _returnvalue_9) 1000.0)))
      (bind _output_get (set `self.Destruction` (`KismetMathLibrary.FClamp` _returnvalue_10)))
      (`InstancedStaticMeshComponent.AddInstance` (`|GetArrayItem` _floor_isms (`KismetMathLibrary.Clamp` (`KismetMathLibrary.FTrunc` (* _returnvalue (+ _output_get (`KismetMathLibrary.RandomFloatInRange` (* _jitter -1.0) _jitter)))) 0 (- _returnvalue 1))) (`KismetMathLibrary.MakeTransform` _returnvalue_9 (`KismetMathLibrary.MakeRotator` 0.0 0.0 (+ (`KismetMathLibrary.RandomFloatInRange` (* _returnvalue_3 -1.0) _returnvalue_3) (* (`KismetMathLibrary.RandomInteger` 4) 90.0))) (`KismetMathLibrary.Conv_DoubleToVector` (* (+ (`KismetMathLibrary.RandomFloatInRange` (* _scale_jitter -1.0) _scale_jitter) 1.0) (`self.MeshScalingFactor`)))))
      (set `self.Instance number` (+ (`self.Instance number`) 1)))))

(event `self.ReceiveBeginPlay`
  (if (not (`self.BuildInConstructionScript`))
    (goto _label)))

(fn `UserConstructionScript`
  (if (`self.BuildInConstructionScript`)
    (`self.Build`)))