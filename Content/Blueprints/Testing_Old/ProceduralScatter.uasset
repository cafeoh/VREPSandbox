(event `Build`
  (bind _plane (`self.Plane`))
  (bind (_min _max) (`StaticMeshComponent.GetLocalBounds` _plane))
  (bind _returnvalue (`SceneComponent.K2_GetComponentScale` _plane))
  (bind _returnvalue_2 (`KismetMathLibrary.FTrunc` (.x (/ (+ (* (* _min _returnvalue) -1.0) (* _max _returnvalue)) (`self.Spacing`)))))
  (bind _returnvalue_3 (`KismetMathLibrary.FTrunc` (.y (/ (+ (* (* _min _returnvalue) -1.0) (* _max _returnvalue)) (`self.Spacing`)))))
  (bind _returnvalue_4 (`AddComponent|NODE_AddInstancedStaticMeshComponent-1` :`RelativeTransform` (`KismetMathLibrary.InvertTransform` (`KismetMathLibrary.MakeTransform` (0.0 0.0 0.0) (struct) _returnvalue)) :!label _label))
  (`StaticMeshComponent.SetStaticMesh` _returnvalue_4 (`self.MeshInstance`))
  (`PrimitiveComponent.SetMaterial` _returnvalue_4 0 (`self.Material`))
  (for _index (range (+ _returnvalue_2 1))
    (for _index_2 (range (+ _returnvalue_3 1))
      (`InstancedStaticMeshComponent.AddInstance` _returnvalue_4 (`KismetMathLibrary.MakeTransform` (+ (* (+ (0.0 0.0 0.0) (`KismetMathLibrary.MakeVector` (`KismetMathLibrary.Conv_IntToDouble` _index) (`KismetMathLibrary.Conv_IntToDouble` _index_2))) (`self.Spacing`)) (* _min _returnvalue)) (struct) (* (1.0 1.0 1.0) (`self.MeshScalingFactor`))))))
  (`KismetSystemLibrary.PrintString` (`KismetStringLibrary.Concat_StrStr` (`KismetStringLibrary.Conv_IntToString` _returnvalue_2) " x " (`KismetStringLibrary.Conv_IntToString` _returnvalue_3) " : " (`KismetStringLibrary.Conv_IntToString` (* _returnvalue_2 _returnvalue_3))) true true (struct :`R` 0.640625 :`B` 0.51519 :`A` 1.0) 1000.0))

(event `self.ReceiveBeginPlay`
  (if (not (`self.BuildInConstructionScript`))
    (goto _label)))

(fn `UserConstructionScript`
  (if (`self.BuildInConstructionScript`)
    (`self.Build`)))