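; LiquidUnitO models a liquid mixture as an array of typed liquid objects with a total Quantity.
; AddLiquid merges matching types or constructs new entries, refreshing the material only on a merge.
; PourIntoContainer adds each liquid to a recipient, scaled by its quantity, then PourOut lowers only the source's total.
; A dynamic MI_Liquid instance receives MRT and Color from quantity-weighted sums, multiplied by total Quantity.
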(fn `AddLiquid`
  (params (NewParam :type "/Game/Blueprints/LWater Object Reference (by ref)") (NewParam1 :type "Float (double-precision)"))
  (locals (LiquidAlreadyPresent :type Boolean))
  (bind _returnvalue (`GameplayStatics.GetObjectClass` NewParam))
  (set `self.Quantity` (+ NewParam1 (`self.Quantity`)))
  (for _array_element (`self.Liquids`)
    (if (`|EnumEquality` (`/Game/Blueprints/LWater.Type` NewParam) (`/Game/Blueprints/LWater.Type` _array_element))
      (`/Game/Blueprints/LWater.AddQuantity` _array_element NewParam1)
      (`self.UpdateMaterialInstance`)
      (set `local.LiquidAlreadyPresent` true)
      (`KismetSystemLibrary.PrintString` null (`KismetStringLibrary.Concat_StrStr` "LiquidUnit name : " (`KismetSystemLibrary.GetDisplayName` self)))
      (break)))
  (if (not (`local.LiquidAlreadyPresent`))
    (`KismetSystemLibrary.PrintString` null (`KismetStringLibrary.Concat_StrStr` "Class : [" (`KismetSystemLibrary.GetClassDisplayName` _returnvalue) "]"))
    (bind _returnvalue_2 (`|GenericCreateObject` _returnvalue self NewParam1))
    (`KismetArrayLibrary.Array_Add` (`self.Liquids`) _returnvalue_2)))

(fn `PourIntoContainer`
  (params (Recipient :type "/Game/Blueprints/LiquidUnitO Object Reference (by ref)") (Quantity :type "Float (double-precision)"))
  (for _array_element (`self.Liquids`)
    (`self.AddLiquid` Recipient _array_element (* (/ (`/Game/Blueprints/LWater.Quantity` _array_element) 1.0) Quantity)))
  (`self.PourOut` Quantity))

(fn `PourOut`
  (params (QuantityOut :type "Float (double-precision)"))
  (set `self.Quantity` (- (`self.Quantity`) QuantityOut)))

(fn `UpdateMaterialInstance`
  (returns (MaterialInstance :type "MaterialInstanceDynamic Object Reference"))
  (locals (MRT :type "Vector Structure") (Color :type "Vector Structure"))
  (bind _materialinstance (`self.MaterialInstance`))
  (bind _quantity (`self.Quantity`))
  (`/Engine/EditorBlueprintResources/StandardMacros.IsValid` (`self.MaterialInstance`)
    (:`Is Valid`
      _)
    (:`Is Not Valid`
      (bind _returnvalue (`KismetMaterialLibrary.CreateDynamicMaterialInstance` self "/Game/Materials/MI_Liquid.MI_Liquid"))
      (set `self.MaterialInstance` _returnvalue)))
  (for _array_element (`self.Liquids`)
    (bind _quantity_2 (`/Game/Blueprints/LWater.Quantity` _array_element))
    (set `local.MRT` (+ (* (`/Game/Blueprints/LWater.MRT` _array_element) _quantity_2) (`local.MRT`)))
    (set `local.Color` (+ (* (`KismetMathLibrary.Conv_LinearColorToVector` (`/Game/Blueprints/LWater.Color` _array_element)) _quantity_2) (`local.Color`))))
  (`MaterialInstanceDynamic.SetVectorParameterValue` _materialinstance "MRT" (`KismetMathLibrary.Conv_VectorToLinearColor` (* (`local.MRT`) _quantity)))
  (`MaterialInstanceDynamic.SetVectorParameterValue` _materialinstance "Color" (`KismetMathLibrary.Conv_VectorToLinearColor` (* (`local.Color`) _quantity)))
  (return _materialinstance))