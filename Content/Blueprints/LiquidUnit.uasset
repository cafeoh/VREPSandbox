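; LiquidUnit models a mixture of liquid objects that can be added to, poured into another container or poured out.
; AddLiquid merges liquids by class or constructs a new entry, and each change re-sums the total Quantity.
; Pouring out scales each liquid's share, while pouring into a container passes liquids on through the recipient's AddLiquid.
; A dynamic MI_Liquid material shows the quantity-weighted average Color and MRT, refreshed only when an existing liquid gains quantity.
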(fn UpdateMaterialInstance
  (bind _quantity (Variables|Default|GetQuantity))
  (Utilities|IsValid (Variables|Default|GetMaterialInstance)
    (:Is%20Valid
      _)
    (:Is%20Not%20Valid
      (bind _returnvalue (Rendering|Material|CreateDynamicMaterialInstance self "/Game/Materials/MI_Liquid.MI_Liquid" :!class /Script/Engine.KismetMaterialLibrary))
      (Variables|Default|SetMaterialInstance _returnvalue)))
  (for _array_element (Variables|Default|GetLiquids)
    (LocalVariables|SetMRT (+ (* (Variables|/Game/Blueprints/LWater.LWater_C|GetMRT _array_element) (Variables|/Game/Blueprints/LWater.LWater_C|GetQuantity _array_element)) (LocalVariables|GetMRT)))
    (LocalVariables|SetColor (+ (* (Math|Conversions|ToVector(LinearColor) (Variables|/Game/Blueprints/LWater.LWater_C|GetColor _array_element)) (Variables|/Game/Blueprints/LWater.LWater_C|GetQuantity _array_element)) (LocalVariables|GetColor))))
  (Rendering|Material|SetVectorParameterValue (Variables|Default|GetMaterialInstance) "MRT" (Math|Conversions|ToLinearColor(Vector) (/ (LocalVariables|GetMRT) _quantity)) :!class /Script/Engine.MaterialInstanceDynamic)
  (Rendering|Material|SetVectorParameterValue (Variables|Default|GetMaterialInstance) "Color" (Math|Conversions|ToLinearColor(Vector) (/ (LocalVariables|GetColor) _quantity)) :!class /Script/Engine.MaterialInstanceDynamic)
  (return (Variables|Default|GetMaterialInstance)))

(fn PourIntoContainer
  (params (Recipient :type Liquid%20Unit%20Object%20Reference%20%28by%20ref%29) (Quantity :type Float%20%28single-precision%29))
  (for _array_element (Variables|Default|GetLiquids)
    (CallFunction|AddLiquid Recipient _array_element (* (/ (Variables|/Game/Blueprints/LWater.LWater_C|GetQuantity _array_element) (Variables|Default|GetQuantity)) Quantity))
    (Variables|/Game/Blueprints/LWater.LWater_C|SetQuantity _array_element (- (Variables|/Game/Blueprints/LWater.LWater_C|GetQuantity _array_element) (* (/ (Variables|/Game/Blueprints/LWater.LWater_C|GetQuantity _array_element) (Variables|Default|GetQuantity)) Quantity))))
  (CallFunction|UpdateQuantity))

(fn PourOut
  (params (QuantityOut :type Float%20%28single-precision%29))
  (for _array_element (Variables|Default|GetLiquids)
    (Variables|/Game/Blueprints/LWater.LWater_C|SetQuantity _array_element (|((({EA9AAF71-460E-2104-2C34-52BC6AB0ECAF}-QOut)/{EA9AAF71-460E-2104-2C34-52BC6AB0ECAF})*LiQuant) QuantityOut (Variables|/Game/Blueprints/LWater.LWater_C|GetQuantity _array_element))))
  (CallFunction|UpdateQuantity))

(fn AddLiquid
  (params (NewParam :type L%20Water%20Object%20Reference%20%28by%20ref%29) (NewParam1 :type Float%20%28single-precision%29))
  (bind _array_element (Utilities|Array|ForEachLoopwithBreak (Variables|Default|GetLiquids) :!label _label)
    (:LoopBody
      (if (== (Utilities|GetClass NewParam) (Utilities|GetClass _array_element))
        (Default|AddQuantity _array_element NewParam1)
        (CallFunction|UpdateMaterialInstance)
        (LocalVariables|SetLiquidAlreadyPresent true)
        (goto _label Break)))
    (:Completed
      (if (LocalVariables|GetLiquidAlreadyPresent)
        _
        (else
          (bind _returnvalue (Game|ConstructObjectfromClass (Utilities|GetClass NewParam) self NewParam1))
          (Utilities|Array|Add (Variables|Default|GetLiquids) _returnvalue)))
      (CallFunction|UpdateQuantity))))

(fn UpdateQuantity
  (for _array_element (Variables|Default|GetLiquids)
    (LocalVariables|SetNewQuantity (+ (LocalVariables|GetNewQuantity) (Variables|/Game/Blueprints/LWater.LWater_C|GetQuantity _array_element))))
  (Variables|Default|SetQuantity (LocalVariables|GetNewQuantity)))