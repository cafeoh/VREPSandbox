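; SkullBP is a physics-driven skull enemy that chases the player's VR camera and can be damaged and killed.
; Each Tick, opposing offset forces turn it toward the camera and upright, while extra forward-point thrust pulls it in.
; Fast spinning sets Stunness, which weakens thrust, dims the material glow and decays when spinning slows.
; At zero health it stops steering, enables gravity, loses its glow and shrinks away as its short lifespan expires.
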(event `self.ReceiveTick`
  (params (DeltaSeconds :type "Float (single-precision)"))
  (bind _returnvalue (`self.GetLifeSpan`))
  (bind _speed (`self.GetRotationalPullDistance`))
  (bind _skull (`self.Skull`))
  (bind _returnvalue_2 (* (`KismetMathLibrary.MakeVector` 0.0 0.0 1.0) (`self.GetRotationalSpeed`)))
  (bind _returnvalue_3 (`SceneComponent.K2_GetComponentLocation` _skull))
  (bind _returnvalue_4 (`SceneComponent.GetForwardVector` _skull))
  (bind _returnvalue_5 (* _speed -1.0))
  (bind _returnvalue_6 (* (`SceneComponent.GetUpVector` _skull) 5.0))
  (`|ExecutionSequence`
    (:`then_0`
      (`MaterialInstanceDynamic.SetScalarParameterValue` (`self.DynamicMaterial`) "Glow Strength" (`KismetMathLibrary.FClamp` (- 1.0 (`self.Stunness`))))
      (if (!= _returnvalue 0.0)
        (`SceneComponent.SetWorldScale3D` (`self.Skull`) (`KismetMathLibrary.Conv_DoubleToVector` (`KismetMathLibrary.FClamp` _returnvalue)))))
    (:`then_1`
      (if (`self.Alive`)
        (bind _asvive_pawn_character (cast `/Game/VRExpansion/Vive/Vive_PawnCharacter` (`GameplayStatics.GetPlayerPawn` 0)))
        (bind _returnvalue_7 (`KismetMathLibrary.Normal` (- (`SceneComponent.K2_GetComponentLocation` (`VRBaseCharacter.VRReplicatedCamera` _asvive_pawn_character)) _returnvalue_3)))
        (bind _returnvalue_8 (* _returnvalue_7 (`self.GetRotationalSpeed`)))
        (`PrimitiveComponent.AddForceAtLocation` _skull (* _returnvalue_8 -1.0) (+ (* _returnvalue_4 _returnvalue_5) _returnvalue_3) "None")
        (`PrimitiveComponent.AddForceAtLocation` _skull (+ _returnvalue_8 (* _returnvalue_7 (* (- 1.0 (`self.Stunness`)) (`self.GetSpeed`)))) (+ (* _returnvalue_4 _speed) _returnvalue_3) "None")
        (`PrimitiveComponent.AddForceAtLocation` _skull _returnvalue_2 (+ _returnvalue_3 (* _returnvalue_6 _speed)) "None")
        (`PrimitiveComponent.AddForceAtLocation` _skull (* _returnvalue_2 -1.0) (+ _returnvalue_3 (* _returnvalue_6 _returnvalue_5)) "None")
        (bind _returnvalue_9 (`PrimitiveComponent.GetPhysicsAngularVelocity` _skull "None"))
        (if (>= (`KismetMathLibrary.VSize` _returnvalue_9) 500.0)
          (set `self.Stunness` 1.0)
          (else
            (set `self.Stunness` (* (`self.Stunness`) 0.97))))))))

(event `self.ReceiveAnyDamage`
  (params (Damage :type "Float (single-precision)") (DamageType :type "DamageType Object Reference") (InstigatedBy :type "Controller Object Reference") (DamageCauser :type "Actor Object Reference"))
  ;[0.04167 0 0.002191] Damage and Death
  (if (`self.Alive`)
    (bind _output_get (set `self.Health` (- (`self.Health`) Damage)))
    (if (<= _output_get 0.0)
      (set `self.Alive` false)
      (`PrimitiveComponent.SetEnableGravity` (`self.Skull`) true)
      (set `self.Stunness` 2.0)
      (`self.SetLifeSpan` 2.0))))

(fn `UserConstructionScript`
  (bind _returnvalue (`PrimitiveComponent.CreateDynamicMaterialInstance` (`self.Skull`) 0 "/Game/Geometry/Skull/MI_Skull.MI_Skull"))
  (set `self.DynamicMaterial` _returnvalue))