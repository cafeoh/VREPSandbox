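; PotSkullBP is a flying skull enemy that homes in on the VR player's camera using physics impulses.
; Tick applies offset impulses to turn and pull it toward the player and keep it upright, with stun countering the forward thrust.
; Fast spinning triggers a decaying stun, which also drives the material and dims the light.
; Lethal damage stops homing, enables gravity, and starts a short lifespan that shrinks the skull away.
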(event `self.ReceiveTick`
  (params (DeltaSeconds :type "Float (single-precision)"))
  (bind _returnvalue (`self.GetLifeSpan`))
  (bind _returnvalue_2 (`KismetMathLibrary.FMin` DeltaSeconds 0.1))
  (bind _skull (`self.Skull`))
  (bind _stunness (`self.Stunness`))
  (bind _returnvalue_3 (`SceneComponent.K2_GetComponentLocation` _skull))
  (bind _returnvalue_4 (`SceneComponent.GetForwardVector` _skull))
  (bind _returnvalue_5 (`SceneComponent.GetUpVector` _skull))
  (bind _returnvalue_6 (* (`self.GetRotationalSpeed`) _returnvalue_2))
  (bind _returnvalue_7 (* _returnvalue_6 -1.0))
  (`|ExecutionSequence`
    (:`then_0`
      (`MaterialInstanceDynamic.SetScalarParameterValue` (`self.DynamicMaterial`) "Stun" _stunness)
      (`LightComponent.SetIntensity` (`self.PointLight`) (* (- 1.0 _stunness) 5000.0))
      (if (!= _returnvalue 0.0)
        (`SceneComponent.SetWorldScale3D` (`self.Skull`) (`KismetMathLibrary.Conv_DoubleToVector` (`KismetMathLibrary.FClamp` _returnvalue)))))
    (:`then_1`
      (if (`self.Alive`)
        (bind _asvive_pawn_character (cast `/Game/VRExpansion/Vive/Vive_PawnCharacter` (`GameplayStatics.GetPlayerPawn` 0)))
        (bind _returnvalue_8 (* (`KismetMathLibrary.Normal` (- (`SceneComponent.K2_GetComponentLocation` (`VRBaseCharacter.VRReplicatedCamera` _asvive_pawn_character)) _returnvalue_3)) (* (`self.GetSpeed`) _returnvalue_2)))
        (`PrimitiveComponent.AddImpulseAtLocation` _skull (* _returnvalue_8 (* (`self.Stunness`) -1.0)) (+ (* _returnvalue_4 _returnvalue_7) _returnvalue_3) "None")
        (`PrimitiveComponent.AddImpulseAtLocation` _skull _returnvalue_8 (+ (* _returnvalue_4 _returnvalue_6) _returnvalue_3) "None")
        (`PrimitiveComponent.AddImpulseAtLocation` _skull (0.0 0.0 100.0) (+ _returnvalue_3 (* _returnvalue_5 _returnvalue_6)) "None")
        (`PrimitiveComponent.AddImpulseAtLocation` _skull (0.0 0.0 -100.0) (+ _returnvalue_3 (* _returnvalue_5 _returnvalue_7)) "None")
        (bind _returnvalue_9 (`PrimitiveComponent.GetPhysicsAngularVelocity` _skull "None"))
        (if (>= (`KismetMathLibrary.VSize` _returnvalue_9) 500.0)
          (set `self.Stunness` 1.0)
          (else
            (set `self.Stunness` (* (`self.Stunness`) 0.97))))))))

(event `self.ReceiveAnyDamage`
  (params (Damage :type "Float (single-precision)") (DamageType :type "DamageType Object Reference") (InstigatedBy :type "Controller Object Reference") (DamageCauser :type "Actor Object Reference"))
  ;[0.04167 0 0.002191] Damage and Death
  (if (`self.Alive`)
    (bind _output_get (set `self.Health` (- (`self.Health`) Damage)))
    (if (<= _output_get 0.0)
      (set `self.Alive` false)
      (`PrimitiveComponent.SetEnableGravity` (`self.Skull`) true)
      (set `self.Stunness` 2.0)
      (`self.SetLifeSpan` 2.0))))

(fn `UserConstructionScript`
  (bind _returnvalue (`PrimitiveComponent.CreateDynamicMaterialInstance` (`self.Skull`) 0 "/Game/Geometry/Skull/MI_PotSkull.MI_PotSkull"))
  (set `self.DynamicMaterial` _returnvalue))